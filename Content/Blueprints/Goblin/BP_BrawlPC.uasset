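; BP_BrawlPC is a player controller that starts in game-only input and handles pausing through the Pause input action.
; The action toggles between PauseGame and ResumeGame based on the current paused state.
; Pausing creates a new WBP_PauseMenu each time, passes it the controller, focuses its Continue button and shows the cursor under game-and-UI input.
; Resuming unpauses, removes the menu, hides the cursor and restores game-only input.
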(event EventBeginPlay
  (Input|SetInputModeGameOnly self))

(event Input|ActionEvents|InputActionPause
  (params (Key :type Key%20Structure :default "None"))
  (:Pressed
    (if (Game|IsGamePaused)
      (CallFunction|ResumeGame)
      (else
        (CallFunction|PauseGame)))))

(fn ConstructionScript)

(fn PauseGame
  (bind _self self)
  (Input|SetInputModeGameandUI self 0 "DoNotLock" true)
  (Game|SetGamePaused true)
  (bind _returnvalue (UserInterface|CreateWidget "/Game/Blueprints/Menus/WBP_PauseMenu.WBP_PauseMenu_C" _self))
  (bind _output_get (Variables|Default|SetPauseMenu _returnvalue))
  (Default|SetPlayerControllerPaused _output_get _self)
  (UserInterface|Viewport|AddtoViewport _output_get 0)
  (Widget|SetKeyboardFocus (Variables|/Game/Blueprints/Menus/WBP_PauseMenu.WBP_PauseMenu_C|GetContinue _output_get))
  (Variables|Default|SetbShowMouseCursor true))

(fn ResumeGame
  (Input|SetInputModeGameOnly self)
  (Game|SetGamePaused false)
  (Widget|RemovefromParent (Variables|Default|GetPauseMenu))
  (Variables|Default|SetbShowMouseCursor false))