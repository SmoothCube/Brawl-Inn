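; BP_WaiterDoor is a door actor that swings open around its yaw axis and closes itself, with OpenDoor called from outside this graph.
; A timeline drives the yaw as an offset from the rotation stored at BeginPlay, so it works at any placed orientation.
; When forward playback finishes, a short retriggerable delay runs before CloseDoor reverses the same timeline.
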(event Custom|CloseDoor
  (bind (_direction _rotation) (Timeline|Timeline_0 Reverse)
    (:Update
      (Transformation|SetActorRotation (Math|Rotator|MakeRotator 0.0 0.0 (+ _rotation (.yaw (Variables|Default|GetSpawnRotation))))))
    (:Finished
      (switch Utilities|FlowControl|Switch|SwitchonETimelineDirection _direction
        (:Forward
          (Utilities|FlowControl|RetriggerableDelay 0.2)
          (CallFunction|CloseDoor))))))

(event Custom|OpenDoor
  (bind (_direction _rotation) (Timeline|Timeline_0 Play)
    (:Update
      (Transformation|SetActorRotation (Math|Rotator|MakeRotator 0.0 0.0 (+ _rotation (.yaw (Variables|Default|GetSpawnRotation))))))
    (:Finished
      (switch Utilities|FlowControl|Switch|SwitchonETimelineDirection _direction
        (:Forward
          (Utilities|FlowControl|RetriggerableDelay 0.2)
          (CallFunction|CloseDoor))))))

(event EventBeginPlay
  (Variables|Default|SetSpawnRotation (Transformation|GetActorRotation)))

(fn ConstructionScript)