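; BP_Prop is a physics prop built on a destructible component that gets pushed around by characters and radial damage.
; On BeginPlay it picks a random destructible mesh from its Meshes array.
; Overlapping a Character_B applies an impulse scaled from that character's movement velocity.
; Radial damage applies an impulse away from the origin, scaled by damage and distance from it.
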(event OnComponentBeginOverlap(Destructible)
  (params (OverlappedComponent :type Primitive%20Component%20Object%20Reference) (OtherActor :type Actor%20Object%20Reference) (OtherComp :type Primitive%20Component%20Object%20Reference) (OtherBodyIndex :type Integer) (bFromSweep :type Boolean) (SweepResult :type Hit%20Result%20Structure%20%28by%20ref%29))
  (bind (_ascharacter_b _bsuccess) (Utilities|Casting|CastToCharacter_B OtherActor))
  (if _bsuccess
    (Physics|AddImpulse (Variables|Default|GetDestructible) (* (Variables|/Script/Engine.MovementComponent|GetVelocity (Variables|/Script/Engine.Character|GetCharacterMovement _ascharacter_b)) (Variables|Default|GetPushStrength)) "None" false)))

(event EventBeginPlay
  (Class|DestructibleComponent|SetDestructibleMesh (Variables|Default|GetDestructible) (Utilities|Array|Get(acopy) (Variables|Default|GetMeshes) (Math|Random|RandomInteger (Utilities|Array|Length (Variables|Default|GetMeshes))))))

(event Game|Damage|EventRadialDamage
  (params (DamageReceived :type Float%20%28single-precision%29) (DamageType :type Damage%20Type%20Object%20Reference) (Origin :type Vector :default "0, 0, 0") (HitInfo :type Hit%20Result%20Structure%20%28by%20ref%29) (InstigatedBy :type Controller%20Object%20Reference) (DamageCauser :type Actor%20Object%20Reference))
  (Physics|AddImpulse (Variables|Default|GetDestructible) (* (- (Transformation|GetWorldLocation (Variables|Default|GetDestructible)) Origin) (* (Variables|Default|GetBarrelPushStrength) DamageReceived)) "None" false))

(fn ConstructionScript)