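; A nav link proxy that swings the bar door open when an AI agent reaches its smart link.
; On BeginPlay it caches the first StaticMeshActor tagged BarDoor.
; Reaching the link plays a timeline that drives the door's relative yaw, then reverses it after a short delay to close the door again.
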(event EventBeginPlay
  (bind _outactors (Actor|GetAllActorsOfClasswithTag "/Script/Engine.StaticMeshActor" "BarDoor"))
  (if (> (Utilities|Array|Length _outactors) 0)
    (bind _asstatic_mesh_actor (Utilities|Casting|CastToStaticMeshActor (Utilities|Array|Get(acopy) _outactors)))
    (Variables|Default|SetDoor _asstatic_mesh_actor)))

(event EventSmartLinkReached
  (params (Agent :type Actor%20Object%20Reference) (Destination :type Vector%20%28by%20ref%29 :default "0, 0, 0"))
  (Utilities|IsValid (Variables|Default|GetDoor)
    (:Is%20Valid
      (bind (_direction _rotation) (Timeline|OpenDoor Play)
        (:Update
          (Transformation|SetRelativeRotation (Variables|/Script/Engine.Actor|GetRootComponent (Variables|Default|GetDoor)) (Math|Rotator|MakeRotator 0.0 0.0 _rotation) false false))
        (:Finished
          (switch Utilities|FlowControl|Switch|SwitchonETimelineDirection _direction
            (:Forward
              (Utilities|FlowControl|Delay 0.5)
              (Timeline|OpenDoor Reverse))))))))

(fn ConstructionScript)