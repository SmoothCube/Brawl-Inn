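; Menu game mode that controls the intro camera flow between level load and the start of play.
; After level load, it points view targets at the first CameraActor tagged "Intro".
; The play button event plays the Intro level sequence and disables controller inputs.
; When the sequence finishes, view targets cut to BP_SequenceCamera without blending and inputs are re-enabled.
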(event Custom|OnIntroFinished
  (bind _returnvalue (Actor|GetActorOfClass "/Game/Blueprints/System/Camera/BP_SequenceCamera.BP_SequenceCamera_C"))
  (Class|GameModeB|UpdateViewTargets _returnvalue 0.0 false)
  (Class|GameModeB|EnableControllerInputs))

(event EventPlayButtonClicked
  (|CallParentFunction)
  (bind _returnvalue (Sequencer|Player|CreateLevelSequencePlayer "/Game/Sequences/MenuMap_v3/Intro.Intro"))
  (Sequencer|Player|Play _returnvalue :!class /Script/MovieScene.MovieSceneSequencePlayer)
  (EventDispatchers|AssignOnFinished _returnvalue (delegate Custom|OnIntroFinished))
  (Class|GameModeB|DisableControllerInputs))

(event EventPostLevelLoad
  (|CallParentFunction)
  (bind _outactors (Actor|GetAllActorsOfClasswithTag "/Script/Engine.CameraActor" "Intro"))
  (if (Utilities|Array|IsValidIndex _outactors)
    (bind _ascamera_actor (Utilities|Casting|CastToCameraActor (Utilities|Array|Get(acopy) _outactors)))
    (Class|GameModeB|UpdateViewTargets _ascamera_actor 0.0 false)))

(event EventTick
  (params (DeltaSeconds :type Float%20%28single-precision%29)))

(fn ConstructionScript)