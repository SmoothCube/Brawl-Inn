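; BP_WaiterLink is a smart nav link that opens the bar door when an AI agent reaches it.
; On BeginPlay it caches the BP_BarDoor found by GetActorOfClass, so it needs no manual reference.
; When the smart link is reached, it calls OpenDoor if that door is valid, then passes the event on to the parent.
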(event EventBeginPlay
  (|CallParentFunction)
  (bind _returnvalue (Actor|GetActorOfClass "/Game/Blueprints/Objects/BP_BarDoor.BP_BarDoor_C"))
  (Variables|Default|SetDoor _returnvalue))

(event Collision|EventActorBeginOverlap
  (params (OtherActor :type Actor%20Object%20Reference))
  (|CallParentFunction OtherActor) ; This node is disabled and will not be called.\nDrag off pins to build functionality.
)

(event EventTick
  (params (DeltaSeconds :type Float%20%28single-precision%29))
  (|CallParentFunction DeltaSeconds) ; This node is disabled and will not be called.\nDrag off pins to build functionality.
)

(event EventSmartLinkReached
  (params (Agent :type Actor%20Object%20Reference) (Destination :type Vector%20%28by%20ref%29 :default "0, 0, 0"))
  (bind _door (Variables|Default|GetDoor))
  (Utilities|IsValid _door
    (:Is%20Valid
      (Default|OpenDoor _door)
      (|CallParentFunction Agent Destination))
    (:Is%20Not%20Valid
      (|CallParentFunction Agent Destination))))

(fn ConstructionScript
  (|CallParentFunction))